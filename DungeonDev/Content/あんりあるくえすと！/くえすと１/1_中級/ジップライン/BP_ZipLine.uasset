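; Zip line actor that carries the player along an editable spline in either direction.
; The construction script builds spline-mesh cable segments and moves the end trigger to the last spline point.
; Overlapping either trigger signals the player through interface messages and plays a timeline forward or in reverse, setting their transform below the line and flipping yaw for reverse rides.
; Finishing or InterruptZipLine releases the player.
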(event OnComponentBeginOverlap(Start_collision)
  (params (OverlappedComponent :type Primitive%20Component%20Object%20Reference) (OtherActor :type Actor%20Object%20Reference) (OtherComp :type Primitive%20Component%20Object%20Reference) (OtherBodyIndex :type Integer) (bFromSweep :type Boolean) (SweepResult :type Hit%20Result%20Structure%20%28by%20ref%29))
  ;[1 1 1] Player判定
  (bind _output_get (Variables|Default|SetOther%20Actor OtherActor))
  (bind _isplayer (Class|BPIZiplinePlayer|BPifIsPlayer(Message) _output_get))
  ;[1 1 1] ZipLine使用中か判定
  (if (and _isplayer (not (Variables|Default|GetRunning_ZipLine)))
    ;[1 1 1] 掴まり処理
    (bind _output_get_2 (Variables|Default|SetRunning_ZipLine true))
    (Class|BPIZiplinePlayer|BPifGrabZipLine(Message) (Variables|Default|GetOther%20Actor) _output_get_2)
    ;[1 1 1] Splineの向き判定
    (Variables|Default|SetStart%20->%20End true)
    (bind _rate (Timeline|ZipLine_Running PlayFromStart) ; キャラクターの変移
      (:Update
        ;[1 1 1] TimeLine Play Rate
        (Components|Timeline|SetPlayRate (Variables|Default|GetZipLine_Running) (Variables|Default|GetTimeLine_Play_Rate))
        ;[1 1 1] Spline上の距離取得
        (Variables|Default|SetDistance (* (Spline|GetSplineLength (Variables|Default|GetSpline)) _rate))
        (if (Variables|Default|GetStart%20->%20End)
          ;[1 1 1] キャラクターの向き取得（Start->End）
          (Variables|Default|SetSpline_Move_Rotation (Spline|GetRotationatDistanceAlongSpline (Variables|Default|GetSpline) (Variables|Default|GetDistance) "World"))
          (else
            ;[1 1 1] キャラクターの向き取得（End->Start）
            (Variables|Default|SetSpline_Move_Rotation (Math|Rotator|MakeRotator (.roll (Spline|GetRotationatDistanceAlongSpline (Variables|Default|GetSpline) (Variables|Default|GetDistance) "World")) (.pitch (Spline|GetRotationatDistanceAlongSpline (Variables|Default|GetSpline) (Variables|Default|GetDistance) "World")) (+ (.yaw (Spline|GetRotationatDistanceAlongSpline (Variables|Default|GetSpline) (Variables|Default|GetDistance) "World")) 1.8e+02)))))
        ;[1 1 1] キャラクターの移動
        (Transformation|SetActorTransform (Variables|Default|GetOther%20Actor) (Math|Transform|MakeTransform (Math|Vector|MakeVector (.x (Spline|GetLocationatDistanceAlongSpline (Variables|Default|GetSpline) (Variables|Default|GetDistance) "World")) (.y (Spline|GetLocationatDistanceAlongSpline (Variables|Default|GetSpline) (Variables|Default|GetDistance) "World")) (+ (.z (Spline|GetLocationatDistanceAlongSpline (Variables|Default|GetSpline) (Variables|Default|GetDistance) "World")) -1.2e+02)) (Variables|Default|GetSpline_Move_Rotation) "1.000000,1.000000,1.000000")))
      (:Finished
        ;[1 1 1] 手を放す処理
        (bind _output_get_3 (Variables|Default|SetRunning_ZipLine false))
        (Class|BPIZiplinePlayer|BPifGrabZipLine(Message) (Variables|Default|GetOther%20Actor) _output_get_3)
        (Timeline|ZipLine_Running Stop)))))

(event OnComponentBeginOverlap(End_collision)
  (params (OverlappedComponent :type Primitive%20Component%20Object%20Reference) (OtherActor :type Actor%20Object%20Reference) (OtherComp :type Primitive%20Component%20Object%20Reference) (OtherBodyIndex :type Integer) (bFromSweep :type Boolean) (SweepResult :type Hit%20Result%20Structure%20%28by%20ref%29))
  ;[1 1 1] Player判定
  (bind _output_get (Variables|Default|SetOther%20Actor OtherActor))
  (bind _isplayer (Class|BPIZiplinePlayer|BPifIsPlayer(Message) _output_get))
  ;[1 1 1] ZipLine使用中か判定
  (if (and _isplayer (not (Variables|Default|GetRunning_ZipLine)))
    ;[1 1 1] 掴まり処理
    (bind _output_get_2 (Variables|Default|SetRunning_ZipLine true))
    (Class|BPIZiplinePlayer|BPifGrabZipLine(Message) (Variables|Default|GetOther%20Actor) _output_get_2)
    ;[1 1 1] Splineの向き判定
    (Variables|Default|SetStart%20->%20End false)
    (bind _rate (Timeline|ZipLine_Running ReverseFromEnd) ; キャラクターの変移
      (:Update
        ;[1 1 1] TimeLine Play Rate
        (Components|Timeline|SetPlayRate (Variables|Default|GetZipLine_Running) (Variables|Default|GetTimeLine_Play_Rate))
        ;[1 1 1] Spline上の距離取得
        (Variables|Default|SetDistance (* (Spline|GetSplineLength (Variables|Default|GetSpline)) _rate))
        (if (Variables|Default|GetStart%20->%20End)
          ;[1 1 1] キャラクターの向き取得（Start->End）
          (Variables|Default|SetSpline_Move_Rotation (Spline|GetRotationatDistanceAlongSpline (Variables|Default|GetSpline) (Variables|Default|GetDistance) "World"))
          (else
            ;[1 1 1] キャラクターの向き取得（End->Start）
            (Variables|Default|SetSpline_Move_Rotation (Math|Rotator|MakeRotator (.roll (Spline|GetRotationatDistanceAlongSpline (Variables|Default|GetSpline) (Variables|Default|GetDistance) "World")) (.pitch (Spline|GetRotationatDistanceAlongSpline (Variables|Default|GetSpline) (Variables|Default|GetDistance) "World")) (+ (.yaw (Spline|GetRotationatDistanceAlongSpline (Variables|Default|GetSpline) (Variables|Default|GetDistance) "World")) 1.8e+02)))))
        ;[1 1 1] キャラクターの移動
        (Transformation|SetActorTransform (Variables|Default|GetOther%20Actor) (Math|Transform|MakeTransform (Math|Vector|MakeVector (.x (Spline|GetLocationatDistanceAlongSpline (Variables|Default|GetSpline) (Variables|Default|GetDistance) "World")) (.y (Spline|GetLocationatDistanceAlongSpline (Variables|Default|GetSpline) (Variables|Default|GetDistance) "World")) (+ (.z (Spline|GetLocationatDistanceAlongSpline (Variables|Default|GetSpline) (Variables|Default|GetDistance) "World")) -1.2e+02)) (Variables|Default|GetSpline_Move_Rotation) "1.000000,1.000000,1.000000")))
      (:Finished
        ;[1 1 1] 手を放す処理
        (bind _output_get_3 (Variables|Default|SetRunning_ZipLine false))
        (Class|BPIZiplinePlayer|BPifGrabZipLine(Message) (Variables|Default|GetOther%20Actor) _output_get_3)
        (Timeline|ZipLine_Running Stop)))))

(event Custom|Interrupt%20ZipLine
  ;[1 1 1] 手を放す処理
  (bind _output_get (Variables|Default|SetRunning_ZipLine false :!label _label))
  (Class|BPIZiplinePlayer|BPifGrabZipLine(Message) (Variables|Default|GetOther%20Actor) _output_get)
  (bind _rate (Timeline|ZipLine_Running Stop) ; キャラクターの変移
    (:Update
      ;[1 1 1] TimeLine Play Rate
      (Components|Timeline|SetPlayRate (Variables|Default|GetZipLine_Running) (Variables|Default|GetTimeLine_Play_Rate))
      ;[1 1 1] Spline上の距離取得
      (Variables|Default|SetDistance (* (Spline|GetSplineLength (Variables|Default|GetSpline)) _rate))
      (if (Variables|Default|GetStart%20->%20End)
        ;[1 1 1] キャラクターの向き取得（Start->End）
        (Variables|Default|SetSpline_Move_Rotation (Spline|GetRotationatDistanceAlongSpline (Variables|Default|GetSpline) (Variables|Default|GetDistance) "World"))
        (else
          ;[1 1 1] キャラクターの向き取得（End->Start）
          (Variables|Default|SetSpline_Move_Rotation (Math|Rotator|MakeRotator (.roll (Spline|GetRotationatDistanceAlongSpline (Variables|Default|GetSpline) (Variables|Default|GetDistance) "World")) (.pitch (Spline|GetRotationatDistanceAlongSpline (Variables|Default|GetSpline) (Variables|Default|GetDistance) "World")) (+ (.yaw (Spline|GetRotationatDistanceAlongSpline (Variables|Default|GetSpline) (Variables|Default|GetDistance) "World")) 1.8e+02)))))
      ;[1 1 1] キャラクターの移動
      (Transformation|SetActorTransform (Variables|Default|GetOther%20Actor) (Math|Transform|MakeTransform (Math|Vector|MakeVector (.x (Spline|GetLocationatDistanceAlongSpline (Variables|Default|GetSpline) (Variables|Default|GetDistance) "World")) (.y (Spline|GetLocationatDistanceAlongSpline (Variables|Default|GetSpline) (Variables|Default|GetDistance) "World")) (+ (.z (Spline|GetLocationatDistanceAlongSpline (Variables|Default|GetSpline) (Variables|Default|GetDistance) "World")) -1.2e+02)) (Variables|Default|GetSpline_Move_Rotation) "1.000000,1.000000,1.000000")))
    (:Finished
      (goto _label))))

(event EventBeginPlay)

(event Collision|EventActorBeginOverlap
  (params (OtherActor :type Actor%20Object%20Reference)))

(event EventTick
  (params (DeltaSeconds :type Float%20%28single-precision%29)))

(fn ConstructionScript
  (bind _spline (Variables|Default|GetSpline))
  (bind _returnvalue (Spline|GetSplineLength _spline))
  (bind _returnvalue_2 (Spline|GetTransformatDistanceAlongSpline _spline _returnvalue "World" false))
  (Utilities|FlowControl|Sequence
    (:then_0
      ;[1 1 1] End_collisionの移動
      (Transformation|SetWorldTransform (Variables|Default|GetEnd_collision) (Math|Transform|MakeTransform (.location _returnvalue_2) (Math|Rotator|MakeRotator 0.0 0.0 (.yaw (.rotation _returnvalue_2))) "1.000000,1.000000,1.000000") false false))
    (:then_1
      ;[1 1 1] Splineポイントの取得
      (for _index (range 0 (- (Spline|GetNumberOfSplinePoints (Variables|Default|GetSpline)) 1))
        (Variables|Default|SetIndex _index)
        ;[1 1 1] SplineMeshの追加、StaticMeshの指定
        (bind _returnvalue_3 (AddComponent|AddSplineMeshComponent false))
        (bind _output_get (Variables|Default|SetSpline_Mesh _returnvalue_3))
        (Components|StaticMesh|SetStaticMesh _output_get "/Game/あんりあるくえすと！/くえすと１/1_中級/ジップライン/Cylinder_ブラシ5_StaticMesh.Cylinder_ブラシ5_StaticMesh")
        ;[1 1 1] 伸ばす軸の設定
        (SplineMesh|SetForwardAxis (Variables|Default|GetSpline_Mesh) "Z" true)
        (SplineMesh|SetStartandEnd (Variables|Default|GetSpline_Mesh) (.Location (Spline|GetLocationandTangentatSplinePoint (Variables|Default|GetSpline) (Variables|Default|GetIndex) "Local")) (.Tangent (Spline|GetLocationandTangentatSplinePoint (Variables|Default|GetSpline) (Variables|Default|GetIndex) "Local")) (.Location (Spline|GetLocationandTangentatSplinePoint (Variables|Default|GetSpline) (+ (Variables|Default|GetIndex) 1) "Local")) (.Tangent (Spline|GetLocationandTangentatSplinePoint (Variables|Default|GetSpline) (+ (Variables|Default|GetIndex) 1) "Local")) true :!class /Script/Engine.SplineMeshComponent)))))