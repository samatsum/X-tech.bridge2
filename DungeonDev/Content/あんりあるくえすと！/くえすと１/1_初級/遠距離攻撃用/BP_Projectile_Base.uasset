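; Base projectile actor for ranged attacks that ignores its instigator or owner, plays a launch sound and flies using its ProjectileMovement component.
; Construction applies speed limit and gravity, enabling homing when flagged with a valid Target.
; With a Target, BeginPlay aims velocity at it and sets a short lifespan.
; Hits broadcast OnProjectileImpact, spawn effects, play a sound at world origin and destroy the projectile.
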(event OnComponentHit(SphereCollision)
  (params (HitComponent :type Primitive%20Component%20Object%20Reference) (OtherActor :type Actor%20Object%20Reference) (OtherComp :type Primitive%20Component%20Object%20Reference) (NormalImpulse :type Vector :default "0, 0, 0") (Hit :type Hit%20Result%20Structure%20%28by%20ref%29))
  (Default|CallOnProjectileImpact OtherActor Hit)
  (Effects|SpawnEmitteratLocation (Variables|Impact|GetImpact_Effect) (.Location (Collision|BreakHitResult Hit)))
  (Audio|PlaySoundatLocation (Variables|インパクト|GetImpact_Sound) "0, 0, 0" "0, 0, 0" 1.0 1.0 0.0 0 0 0 0)
  (Actor|DestroyActor))

(event Custom|Rotate%20to%20Target
  (Variables|/Script/Engine.MovementComponent|SetVelocity (Variables|Default|GetProjectileMovement) (* (Math|Vector|GetUnitDirection(Vector) (Transformation|GetActorLocation) (Transformation|GetActorLocation (Variables|ProjectileSettings|GetTarget))) (Variables|ProjectileSettings|GetSpeed))))

(event EventBeginPlay
  (bind _returnvalue (Game|GetInstigator))
  (Audio|PlaySoundatLocation (Variables|Sounds|GetLaunch_Sound) (Transformation|GetActorLocation) "0, 0, 0" 1.0 1.0 0.0 0 0 0 0)
  (Collision|IgnoreActorwhenMoving (Variables|Default|GetSphereCollision) (select (Utilities|IsValid _returnvalue) _returnvalue (Components|GetOwner)) true)
  (Variables|ProjectileSettings|GetTarget
    (:then
      (CallFunction|RotatetoTarget)
      (Actor|SetLifeSpan 1.0))
    (:else)))

(event Collision|EventActorBeginOverlap
  (params (OtherActor :type Actor%20Object%20Reference)))

(event EventTick
  (params (DeltaSeconds :type Float%20%28single-precision%29)))

(fn ConstructionScript
  (bind _projectilemovement (Variables|Default|GetProjectileMovement))
  (Variables|/Script/Engine.ProjectileMovementComponent|SetMaxSpeed _projectilemovement (Variables|ProjectileSettings|GetSpeed))
  (Variables|/Script/Engine.ProjectileMovementComponent|SetMaxSpeed _projectilemovement (Variables|ProjectileSettings|GetMax_Speed))
  (Variables|/Script/Engine.ProjectileMovementComponent|SetProjectileGravityScale _projectilemovement (Variables|ProjectileSettings|GetGravity))
  (Variables|ProjectileSettings|GetTarget
    (:then
      (if (Variables|ProjectileSettings|GetIs_Homing?)
        (Variables|/Script/Engine.ProjectileMovementComponent|SetbIsHomingProjectile _projectilemovement true)
        (Variables|/Script/Engine.ProjectileMovementComponent|SetHomingTargetComponent _projectilemovement (Variables|/Script/Engine.Actor|GetRootComponent (Variables|ProjectileSettings|GetTarget)))))
    (:else)))