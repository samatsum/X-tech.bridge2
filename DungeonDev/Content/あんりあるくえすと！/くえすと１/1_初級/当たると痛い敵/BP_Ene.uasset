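; Enemy actor that hurts the player on contact and can be stomped or damaged to death.
; Body and head overlaps apply damage; the head has a one-second cooldown through Hitted, which also gates stomping.
; Stomping awards score, plays an explosion and destroys the enemy.
; AnyDamage updates capped HP, pushes the ratio to the HP bar widget only on change, and destroys the actor at zero.
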(event OnComponentBeginOverlap(Box)
  (params (OverlappedComponent :type Primitive%20Component%20Object%20Reference) (OtherActor :type Actor%20Object%20Reference) (OtherComp :type Primitive%20Component%20Object%20Reference) (OtherBodyIndex :type Integer) (bFromSweep :type Boolean) (SweepResult :type Hit%20Result%20Structure%20%28by%20ref%29))
  (Utilities|FlowControl|Sequence
    (:then_0
      (|身体に当たったのがプレイヤーキャラならプレイヤーにダメージを与える OtherActor))))

(event OnComponentBeginOverlap(Sphere1)
  (params (OverlappedComponent :type Primitive%20Component%20Object%20Reference) (OtherActor :type Actor%20Object%20Reference) (OtherComp :type Primitive%20Component%20Object%20Reference) (OtherBodyIndex :type Integer) (bFromSweep :type Boolean) (SweepResult :type Hit%20Result%20Structure%20%28by%20ref%29))
  (Utilities|FlowControl|Sequence
    (:then_0
      (|頭に当たったのがプレイヤーキャラならプレイヤーにダメージを与える OtherActor))))

(event OnComponentBeginOverlap(Stomping_Overlap)
  (params (OverlappedComponent :type Primitive%20Component%20Object%20Reference) (OtherActor :type Actor%20Object%20Reference) (OtherComp :type Primitive%20Component%20Object%20Reference) (OtherBodyIndex :type Integer) (bFromSweep :type Boolean) (SweepResult :type Hit%20Result%20Structure%20%28by%20ref%29))
  (bind _asbp_third_person_character (Utilities|Casting|CastToBP_ThirdPersonCharacter OtherActor))
  (if (not (Variables|Default|GetHitted))
    (Variables|Default|SetHitted true)
    (Default|IncreaseScore _asbp_third_person_character 50)
    (Audio|PlaySound2D "/Game/StarterContent/Audio/Explosion01.Explosion01" 1.0 1.0 0.0 0 0)
    (Effects|SpawnEmitteratLocation "/Game/StarterContent/Particles/P_Explosion.P_Explosion" (Transformation|GetActorLocation))
    (Utilities|FlowControl|Delay 0.3)
    (Actor|DestroyActor)))

(event Collision|EventActorBeginOverlap
  (params (OtherActor :type Actor%20Object%20Reference)))

(event EventTick
  (params (DeltaSeconds :type Float%20%28single-precision%29)))

(event Game|Damage|EventAnyDamage
  (params (Damage :type Float%20%28single-precision%29) (DamageType :type Damage%20Type%20Object%20Reference) (InstigatedBy :type Controller%20Object%20Reference) (DamageCauser :type Actor%20Object%20Reference))
  (if (> (Math|Float|Truncate (- (Variables|Default|GetEnemy01_HP) Damage)) (Variables|Default|GetEnemy01_HP_Max))
    (|HP上限だよ！ (Variables|Default|GetEnemy01_HP_Max))
    (else
      (bind _output_get (Variables|Default|SetEnemy01_HP (Math|Float|Truncate (- (Variables|Default|GetEnemy01_HP) Damage))))
      ;[1 1 1] ウィジェット側にある関数で常に計算させるより計算リソース節約できるかも？
      (Variables|/Game/あんりあるくえすと！/くえすと１/1_初級/当たると痛い敵/Enemy_HP_Bar.Enemy_HP_Bar_C|SetEnemy%2001%20Current%20HP%20Ratio (Variables|Default|GetAs%20Enemy%20HP%20Bar) (/ (Math|Conversions|ToFloat(Integer) (Variables|Default|GetEnemy01_HP)) (Math|Conversions|ToFloat(Integer) (Variables|Default|GetEnemy01_HP_Max))))
      (if (<= _output_get 0)
        (Utilities|FlowControl|Delay 0.1)
        (Actor|DestroyActor)
        (else
          (Development|PrintString (Utilities|String|Append "残りEnemy01_HPは、" (Utilities|String|ToString(Integer) _output_get))))))))

(event EventBeginPlay
  (bind _asenemy_hp_bar (Utilities|Casting|CastToEnemy_HP_Bar (UserInterface|GetWidget (Variables|Default|GetEnemy01_HP_Widget))))
  (Variables|Default|SetAs%20Enemy%20HP%20Bar _asenemy_hp_bar)
  ;[1 1 1] ウィジェット側にある関数で常に計算させるより計算リソース節約できるかも？
  (Variables|/Game/あんりあるくえすと！/くえすと１/1_初級/当たると痛い敵/Enemy_HP_Bar.Enemy_HP_Bar_C|SetEnemy%2001%20Current%20HP%20Ratio (Variables|Default|GetAs%20Enemy%20HP%20Bar) (/ (Math|Conversions|ToFloat(Integer) (Variables|Default|GetEnemy01_HP)) (Math|Conversions|ToFloat(Integer) (Variables|Default|GetEnemy01_HP_Max)))))

(fn ConstructionScript)