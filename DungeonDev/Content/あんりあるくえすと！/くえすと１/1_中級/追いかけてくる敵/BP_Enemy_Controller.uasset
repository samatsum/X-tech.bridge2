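; AI Controller for a chasing enemy that runs the BT_Enemy behavior tree on BeginPlay.
; AI Perception target updates are filtered to the first player character and drive the TargetPlayer blackboard key.
; The key holds the player while successfully sensed and is set to an empty object when sensing is lost, feeding the tree its current target.
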(event OnTargetPerceptionUpdated(AIPerception)
  (params (Actor :type Actor%20Object%20Reference) (Stimulus :type AI%20Stimulus%20Structure))
  (if (== Actor (Game|GetPlayerCharacter 0))
    (if (.bSuccessfullySensed (Utilities|Struct|BreakAIStimulus Stimulus))
      (AI|Components|Blackboard|SetValueasObject (Variables|Default|GetBlackboard) (Utilities|Name|MakeLiteralName "TargetPlayer") Actor)
      (else
        (AI|Components|Blackboard|SetValueasObject (Variables|Default|GetBlackboard) (Utilities|Name|MakeLiteralName "TargetPlayer") 0)))))

(event EventBeginPlay
  (AI|RunBehaviorTree "/Game/あんりあるくえすと！/くえすと１/1_中級/追いかけてくる敵/BT_Enemy.BT_Enemy"))

(event EventTick
  (params (DeltaSeconds :type Float%20%28single-precision%29)))

(fn ConstructionScript)