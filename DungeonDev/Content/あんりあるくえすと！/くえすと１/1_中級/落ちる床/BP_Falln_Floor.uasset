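; BP_Falln_Floor is a falling floor tile that drops after the player steps on it and then respawns.
; BeginPlay stores the tile's starting location.
; When BP_ThirdPersonCharacter overlaps the Box trigger, a short delay precedes enabling physics on the Cube so it falls.
; A few seconds later it spawns a fresh copy of itself at the stored location and destroys the fallen instance.
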(event OnComponentBeginOverlap(Box)
  (params (OverlappedComponent :type Primitive%20Component%20Object%20Reference) (OtherActor :type Actor%20Object%20Reference) (OtherComp :type Primitive%20Component%20Object%20Reference) (OtherBodyIndex :type Integer) (bFromSweep :type Boolean) (SweepResult :type Hit%20Result%20Structure%20%28by%20ref%29))
  (Utilities|Casting|CastToBP_ThirdPersonCharacter OtherActor)
  (Utilities|FlowControl|Delay 0.6)
  (Physics|SetSimulatePhysics (Variables|Default|GetCube) true)
  (Utilities|FlowControl|Delay 3.0)
  (Game|SpawnActorfromClass "BP_Falln_Floor_C" (Math|Transform|MakeTransform (Variables|Default|GetInitial_Location) "0, 0, 0" "1.000000,1.000000,1.000000") "Undefined" "MultiplyWithRoot" 0 0)
  (Actor|DestroyActor))

(event EventBeginPlay
  (Variables|Default|SetInitial_Location (Transformation|GetActorLocation)))

(event Collision|EventActorBeginOverlap
  (params (OtherActor :type Actor%20Object%20Reference)))

(event EventTick
  (params (DeltaSeconds :type Float%20%28single-precision%29)))

(fn ConstructionScript)